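; Mordhau Skirmish mod actor that tracks each player's damage to the other team for a scoreboard, swapping in a damage HUD and zeroing the team-kill score change.
; An authority-only looping timer appears to drive CheckDamage, which binds each controller's instigated-damage event.
; In-progress, non-team hits accumulate in a server-only map keyed by PlayerState.
; CheckDamage copies that map into parallel player-order and damage arrays, apparently for replication.
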(event Custom|CheckDamage
  (bind _returnvalue (Game|GetGameState))
  (bind _playerarray (Variables|/Script/Engine.GameStateBase|GetPlayerArray _returnvalue))
  (Variables|Default|SetPlayerStateOrderRep _playerarray)
  (for (_array_element _array_index) _playerarray
    (Utilities|Array|SetArrayElem (Variables|Default|GetDmgRep) _array_index (.Value (Utilities|Map|Find (Variables|Default|GetPlayerDamagesServerOnly) _array_element)) true)
    (bind _asmordhau_player_controller (Utilities|Casting|CastToMordhauPlayerController (Components|GetOwner _array_element)))
    (EventDispatchers|BindEventtoOnInstigatedAnyDamage _asmordhau_player_controller (delegate Custom|CustomEvent_0))))

(event Custom|CustomEvent_0
  (params (Damage :type Float%20%28single-precision%29) (DamageType :type Damage%20Type%20Object%20Reference) (DamagedActor :type Actor%20Object%20Reference) (DamageCauser :type Actor%20Object%20Reference))
  ;[1 1 1] On Damage Dealt
  (if (Utilities|Name|Equal(Name) (Variables|/Script/Engine.GameState|GetMatchState (.AsMordhau%20Game%20State (Utilities|Casting|CastToMordhauGameState (Game|GetGameState)))) "InProgress") ; Not in warmup?
    (bind _asmordhau_character (Utilities|Casting|CastToMordhauCharacter DamageCauser))
    (if (not (== (Variables|/Script/Mordhau.AdvancedCharacter|GetTeam (.AsMordhau%20Character (Utilities|Casting|CastToMordhauCharacter DamagedActor))) (Variables|/Script/Mordhau.AdvancedCharacter|GetTeam _asmordhau_character))) ; is team hit?
      (Utilities|Map|Add (Variables|Default|GetPlayerDamagesServerOnly) (Variables|/Script/Engine.Pawn|GetPlayerState _asmordhau_character) (Math|Float|SelectFloat (+ (.Value (Utilities|Map|Find (Variables|Default|GetPlayerDamagesServerOnly) (Variables|/Script/Engine.Pawn|GetPlayerState _asmordhau_character))) Damage) Damage (.ReturnValue (Utilities|Map|Find (Variables|Default|GetPlayerDamagesServerOnly) (Variables|/Script/Engine.Pawn|GetPlayerState _asmordhau_character))))))))

(event EventBeginPlay
  (bind _asbp_skirmish_game_mode (Utilities|Casting|CastToBP_SkirmishGameMode (Game|GetGameMode)))
  (Variables|/Script/Mordhau.MordhauGameMode|SetTeamKillScoreChange _asbp_skirmish_game_mode 0.0)
  (Variables|/Script/Engine.GameModeBase|SetHUDClass _asbp_skirmish_game_mode "/ScoreboardDMG/HUD_SKM_Dmg.HUD_SKM_Dmg_C")
  (Networking|SwitchHasAuthority
    (:Authority
      (Utilities|Time|SetTimerbyEvent (EventDispatchers|CreateEvent :!event Custom|CheckDamage) 1.0 true))))

(fn ConstructionScript)